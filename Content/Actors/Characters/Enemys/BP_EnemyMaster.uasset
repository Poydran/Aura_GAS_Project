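; Base enemy Blueprint that handles the dissolve visual effect for the enemy and its weapon, apparently on death.
; StartDissolve and StartDissolveWeapon each receive a dynamic material instance and play their own timeline from the start, writing its value to the "Dissolve" scalar parameter.
; Both timelines derive play rate from DeathDespawnTime divided by a constant, so a larger value plays the dissolve faster.
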(event `self.StartDissolve`
  (params (DynamicMaterialInstance :type "MaterialInstanceDynamic Object Reference"))
  (`TimelineComponent.SetPlayRate` (`self.DissolveLine`) (`KismetMathLibrary.SafeDivide` (`self.DeathDespawnTime`) 100.0))
  (bind (_direction _dissolvetimeline) (`Timeline|DissolveLine` :!via `PlayFromStart`)
    (:`Update`
      (`MaterialInstanceDynamic.SetScalarParameterValue` DynamicMaterialInstance "Dissolve" _dissolvetimeline))))

(event `self.StartDissolveWeapon`
  (params (DynamicMaterialInstance :type "MaterialInstanceDynamic Object Reference"))
  (`TimelineComponent.SetPlayRate` (`self.WeaponDissolve`) (`KismetMathLibrary.SafeDivide` (`self.DeathDespawnTime`) 100.0))
  (bind (_direction _dissolvetimeline) (`Timeline|WeaponDissolve` :!via `PlayFromStart`)
    (:`Update`
      (`MaterialInstanceDynamic.SetScalarParameterValue` DynamicMaterialInstance "Dissolve" _dissolvetimeline))))

(fn `UserConstructionScript`)